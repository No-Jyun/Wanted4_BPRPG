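; Player character Blueprint with camera-relative movement, look input, weapon pickup and a montage-driven melee combo attack.
; A collected weapon snaps to the mesh's WeaponPosition socket, and bound event dispatchers relay attack-check begin and end to it.
; Attack input requires a weapon and switches Locomotion to Battle to play the attack montage.
; Further presses queue the next combo section from the current one, and AttackEnd restores Locomotion.
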(event Custom|AttackEnd
  (Variables|Default|SetState_BP "NewEnumerator0"))

(event Custom|OnWeaponCollected
  (params (WeaponActor :type BP%20Weapon%20Object%20Reference))
  ;[0.15 0.000434 0.04825 0.5] 무기 습득 처리
  (Actor|SetOwner WeaponActor self)
  (Transformation|AttachComponentToComponent WeaponActor (Variables|Character|GetMesh) "WeaponPosition" "SnapToTarget" "SnapToTarget" "SnapToTarget" true)
  (Variables|Default|SetWeaponActor WeaponActor)
  (Variables|Default|SetHasWeapon true)
  ;[0.07124 0.15 0.08559 0.5] 공격 판정 시작 이벤트에 함수 등록 (구독)
  (EventDispatchers|BindEventtoAttackCheckBeginEvent (delegate Custom|RaiseAttackCheckBegin))
  ;[0.07124 0.15 0.08559 0.5] 공격 판정 종료 이벤트에 함수 등록 (구독)
  (EventDispatchers|BindEventtoAttackCheckEndEvent (delegate Custom|RaiseAttackCheckEnd)))

(event Custom|OnAttackCheckEnd
  ;[0.06467 0.1434 0.15 0.5] 공격 판정 종료
  (Default|CallAttackCheckEndEvent))

(event Custom|OnAttackCheckBegin
  ;[0.06467 0.1434 0.15 0.5] 공격 판정 시작
  (Default|CallAttackCheckBeginEvent))

(event Custom|RaiseAttackCheckBegin
  (bind _weaponactor (Variables|Default|GetWeaponActor))
  ;[0.07124 0.15 0.08559 0.5] 공격 판정 시작 이벤트에 함수 등록 (구독)
  (Utilities|IsValid _weaponactor
    (:Is%20Valid
      (Default|OnAttackCheckBegin _weaponactor))))

(event Custom|RaiseAttackCheckEnd
  (bind _weaponactor (Variables|Default|GetWeaponActor))
  ;[0.07124 0.15 0.08559 0.5] 공격 판정 종료 이벤트에 함수 등록 (구독)
  (Utilities|IsValid _weaponactor
    (:Is%20Valid
      (Default|OnAttackCheckEnd _weaponactor))))

(event Input|EnhancedActionEvents|EnhancedInputActionIA_Move
  (params (ActionValue :type Vector%202D%20Structure) (ElapsedSeconds :type Float%20%28double-precision%29) (TriggeredSeconds :type Float%20%28double-precision%29) (InputAction :type Input%20Action%20Object%20Reference :default "/Game/Blueprints/Input/Actions/IA_Move.IA_Move"))
  ;[0 0.1448 0.15 0.5] 이동
  (Pawn|Input|AddMovementInput (Math|Vector|GetRightVector (Pawn|GetControlRotation :!class /Script/Engine.Pawn)) (.x ActionValue) false)
  (Pawn|Input|AddMovementInput (Math|Vector|GetForwardVector (Math|Rotator|MakeRotator 0.0 0.0 (.yaw (Pawn|GetControlRotation :!class /Script/Engine.Pawn)))) (.y ActionValue) false))

(event Input|EnhancedActionEvents|EnhancedInputActionIA_View
  (params (ActionValue :type Vector%202D%20Structure) (ElapsedSeconds :type Float%20%28double-precision%29) (TriggeredSeconds :type Float%20%28double-precision%29) (InputAction :type Input%20Action%20Object%20Reference :default "/Game/Blueprints/Input/Actions/IA_View.IA_View"))
  ;[0.000839 0 0.15 0.5] 카메라 회전
  (Pawn|Input|AddControllerYawInput (.x ActionValue)) ; 컨트롤러의 요(Yaw) 회전 추가
  (bind _result (Math|Float|NegateFloat (.y ActionValue))
    (:%20%20
      (Pawn|Input|AddControllerPitchInput _result) ; 컨트롤러의 피치(Pitch) 회전 추가
    )))

(event Input|EnhancedActionEvents|EnhancedInputActionIA_Attack
  (params (ActionValue :type Boolean) (ElapsedSeconds :type Float%20%28double-precision%29) (TriggeredSeconds :type Float%20%28double-precision%29) (InputAction :type Input%20Action%20Object%20Reference :default "/Game/Blueprints/Input/Actions/IA_Attack.IA_Attack"))
  ;[0 0.15 0.01404 0.5] 공격
  (:Started
    (if (Variables|Default|GetHasWeapon)
      ;;[0.08902 0.15 0 0.5] 일반 상태인지 확인
      (switch Utilities|FlowControl|Switch|SwitchonEPlayerState (Variables|Default|GetState_BP)
        (:NewEnumerator0
          (Variables|Default|SetState_BP "NewEnumerator1")
          (Animation|PlayAnimMontage "/Game/Blueprints/Character/AM_Attack.AM_Attack" 1.0 "None"))
        (:NewEnumerator1
          (switch name (Animation|Montage|MontageGetCurrentSection (Components|SkeletalMesh|GetAnimInstance (Variables|Character|GetMesh)) "/Game/Blueprints/Character/AM_Attack.AM_Attack")
            (:Attack1
              (Variables|Default|SetNextCombo "Attack2"))
            (:Attack2
              (Variables|Default|SetNextCombo "Attack3"))
            (:Attack3
              (Variables|Default|SetNextCombo "Attack4"))))))))

(event EventBeginPlay)

(event Collision|EventActorBeginOverlap
  (params (OtherActor :type Actor%20Object%20Reference)))

(event EventTick
  (params (DeltaSeconds :type Float%20%28single-precision%29)))

(fn ConstructionScript)